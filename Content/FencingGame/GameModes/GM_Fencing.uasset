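; Game mode for two-player multiplayer fencing that handles matchmaking within the session, scoring and rematches.
; PostLogin shows a waiting widget to the first player, then links both BP_Fencer pawns as opponents and multicasts the game UI.
; Reported points increment PS_Fencer scores, which PopulateScoreScreens sends to each fencer alongside the opponent's.
; Once two distinct controllers request a rematch, it resets the level, restarts players and re-pairs them.
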(event `self.K2_PostLogin`
  (params (NewPlayer :type "PlayerController Object Reference"))
  (`KismetArrayLibrary.Array_Add` (`self.Players`) NewPlayer)
  (if (> (`KismetArrayLibrary.Array_Length` (`self.Players`)) 1)
    (`KismetSystemLibrary.Delay` 0.1)
    (`self.InitOpponents`)
    (else
      (`KismetSystemLibrary.Delay` 0.1)
      (`self.InitWaitingWidget`))))

(event `InitWaitingWidget`
  (bind _asbp_fencer (cast `/Game/FencingGame/Fencer/BP_Fencer` (`Controller.K2_GetPawn` (`|GetArrayItem` (`self.Players`)))))
  (`/Game/FencingGame/Fencer/BP_Fencer.DisplayWaitingWidget` _asbp_fencer))

(event `InitOpponents`
  (for (_array_element _array_index) (`self.Players`)
    (bind _asbp_fencer (cast `/Game/FencingGame/Fencer/BP_Fencer` (`Controller.K2_GetPawn` _array_element)))
    (`/Game/FencingGame/Fencer/BP_Fencer.MulticastStartGameUI` _asbp_fencer)
    (bind _asbp_fencer_2 (cast `/Game/FencingGame/Fencer/BP_Fencer` (`Controller.K2_GetPawn` (`|GetArrayItem` (`self.Players`) (`KismetMathLibrary.Abs_Int` (- _array_index 1))))))
    (`/Game/FencingGame/Fencer/BP_Fencer.MulticastStartGameUI` _asbp_fencer_2)
    (set `/Game/FencingGame/Fencer/BP_Fencer.Opponent` _asbp_fencer_2 _asbp_fencer)))

(event `ReportReadyForRematch`
  (params (Controller :type "PlayerController Object Reference"))
  (if (not (`KismetArrayLibrary.Array_Contains` (`self.RematchingPlayers`) Controller))
    (bind _returnvalue (`KismetArrayLibrary.Array_Add` (`self.RematchingPlayers`) Controller))
    (if (>= _returnvalue 1)
      (`self.Rematch`))))

(event `Rematch`
  (`self.ResetLevel`)
  (`KismetSystemLibrary.Delay` 0.2)
  (for _array_element (`self.Players`)
    (`self.RestartPlayer` _array_element)
    (bind _asbp_fencer (cast `/Game/FencingGame/Fencer/BP_Fencer` (`Controller.K2_GetPawn` _array_element)))
    (`/Game/FencingGame/Fencer/BP_Fencer.ResetUI` _asbp_fencer))
  (`KismetArrayLibrary.Array_Clear` (`self.RematchingPlayers`))
  (`self.InitOpponents`))

(event `PopulateScoreScreens`
  (for _array_element (`self.Players`)
    (bind _asps_fencer (cast `/Game/FencingGame/GameModes/PS_Fencer` (`Controller.PlayerState` _array_element)))
    (bind _asbp_fencer (cast `/Game/FencingGame/Fencer/BP_Fencer` (`Controller.K2_GetPawn` _array_element)))
    (bind _asps_fencer_2 (cast `/Game/FencingGame/GameModes/PS_Fencer` (`Pawn.PlayerState` (`/Game/FencingGame/Fencer/BP_Fencer.Opponent` _asbp_fencer))))
    (`/Game/FencingGame/Fencer/BP_Fencer.DisplayScore` _asbp_fencer (`/Game/FencingGame/GameModes/PS_Fencer.PlayerScore` _asps_fencer) (`/Game/FencingGame/GameModes/PS_Fencer.PlayerScore` _asps_fencer_2))))

(event `ReportScore`
  (params (Player :type "Controller Object Reference"))
  (bind _asps_fencer (cast `/Game/FencingGame/GameModes/PS_Fencer` (`Controller.PlayerState` Player)))
  (set `/Game/FencingGame/GameModes/PS_Fencer.PlayerScore` (+ (`/Game/FencingGame/GameModes/PS_Fencer.PlayerScore` _asps_fencer) 1) _asps_fencer))

(fn `UserConstructionScript`)