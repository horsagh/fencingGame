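; Networked player character for a one-on-one directional fencing game, with guard, swing, forward/back movement and round-end UI.
; Enhanced Input sends guard and swing requests to the server, which multicasts them into ABP_Fencer state; changing guard can feint a swing.
; On swing connect, the server retries until in range, compares mirrored direction to the opponent's block, then reduces per-zone health and strips armor.
; A kill triggers ragdoll, GM_Fencing scoring and rematch widgets.
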(event `InitAnims`
  ;[1 1 1] Init
  (bind _asabp_fencer (cast `/Game/FencingGame/Fencer/Animations/ABP_Fencer` (`SkeletalMeshComponent.GetAnimInstance` (`self.Mesh`))))
  (set `self.Anim` _asabp_fencer))

(event `SwingConnect`
  ;[1 1 1] Block & Hit
  (`/Engine/EditorBlueprintResources/ActorMacros.Switch Has Authority`
    (:`Authority`
      (`self.ServerTryHit`))))

(event `MulticastGetHit`
  (params (Zone :type "/Game/FencingGame/Fencer/E_Guards Enum" :default "NewEnumerator0") (NewVal :type Integer))
  ;[1 1 1] Block & Hit
  (`BlueprintMapLibrary.Map_Add` (`self.Health`) Zone NewVal)
  (if (<= NewVal 1)
    (`SceneComponent.SetHiddenInGame` (select `/Game/FencingGame/Fencer/E_Guards` Zone :`NewEnumerator0` (`self.ArmorRight`) :`NewEnumerator1` (`self.ArmorUp`) :`NewEnumerator2` (`self.ArmorLeft`)) true false)))

(event `self.ReceiveBeginPlay`
  ;[1 1 1] Init
  (`|ExecutionSequence`
    (:`then_0`
      (`self.InitAnims`))
    (:`then_1`
      (`self.InitInput`))
    (:`then_2`
      (set `self.isLocalPlayer` (== (`GameplayStatics.GetPlayerController` 0) (`self.GetController`))))
    (:`then_3`
      (`self.InitMeshColor`))))

(event `InitInput`
  ;[1 1 1] Init
  (bind _asplayer_controller (cast `PlayerController` (`self.GetController`)))
  (`EnhancedInputSubsystemInterface.AddMappingContext` (pcsubsystem `EnhancedInputLocalPlayerSubsystem` _asplayer_controller) "/Game/FencingGame/Fencer/Input/IMC_Fencer.IMC_Fencer" 0 (struct)))

(event `ServerTryHit`
  (bind _swing (`/Game/FencingGame/Fencer/Animations/ABP_Fencer.Swing` (`self.Anim`)))
  (bind _returnvalue (select `/Game/FencingGame/Fencer/E_Guards` _swing :`NewEnumerator0` "NewEnumerator2" :`NewEnumerator1` "NewEnumerator1" :`NewEnumerator2` "NewEnumerator0" :`NewEnumerator3` "NewEnumerator3" :!type "/Game/FencingGame/Fencer/E_Guards Enum"))
  ;[1 1 1] Block & Hit
  (if (`|EnumEquality` _swing "NewEnumerator3")
    _
    (elif (< (`KismetMathLibrary.Vector_DistanceSquared` (`self.K2_GetActorLocation` (`self.Opponent`)) (`self.K2_GetActorLocation`)) (`KismetMathLibrary.Square` (`self.Range`)))
      (if (`|EnumEquality` _returnvalue (`/Game/FencingGame/Fencer/Animations/ABP_Fencer.BlockingDirection` (`/Game/FencingGame/Fencer/BP_Fencer.Anim` (`self.Opponent`))))
        (`self.MulticastBlocked`)
        (else
          (bind _result (`/Engine/EditorBlueprintResources/StandardMacros.DecrementInt` (`BlueprintMapLibrary.Map_Find` (`/Game/FencingGame/Fencer/BP_Fencer.Health` (`self.Opponent`)) _returnvalue))
            (:`  `
              (if (<= _result 0)
                (if (not (`self.IsDead`))
                  (`self.KillOpponent`)
                  (`self.Die` (`self.Opponent`))
                  (bind _asgm_fencing (cast `/Game/FencingGame/GameModes/GM_Fencing` (`GameplayStatics.GetGameMode`)))
                  (`/Game/FencingGame/GameModes/GM_Fencing.ReportScore` _asgm_fencing (`self.GetController`))
                  (`self.RoundEndClient` self true)
                  (`self.RoundEndClient` (`self.Opponent`) false)
                  (`/Game/FencingGame/GameModes/GM_Fencing.PopulateScoreScreens` _asgm_fencing))
                (else
                  (`self.MulticastGetHit` (`self.Opponent`) _returnvalue _result)
                  (`self.MulticastHit`)))))))
      (else
        (`KismetSystemLibrary.Delay` 0.07)
        (`self.ServerTryHit`)))))

(event `InitMeshColor`
  ;[1 1 1] Init
  (if (`self.isLocalPlayer`)
    (`PrimitiveComponent.SetMaterial` (`self.Mesh`) 0 "/Game/FencingGame/Fencer/Materials/MI_MannyBlue02.MI_MannyBlue02")
    (`PrimitiveComponent.SetMaterial` (`self.Mesh`) 1 "/Game/FencingGame/Fencer/Materials/MI_MannyBlue01.MI_MannyBlue01")))

(event `EnhancedInput|/Game/FencingGame/Fencer/Input/IA_Right`
  (params (ActionValue :type Boolean) (ElapsedSeconds :type "Float (double-precision)") (TriggeredSeconds :type "Float (double-precision)") (InputAction :type "InputAction Object Reference" :default "/Game/FencingGame/Fencer/Input/IA_Right.IA_Right"))
  ;[1 1 1] Input
  (:`Triggered`
    (`self.DirectionalInput` "NewEnumerator0")))

(event `DirectionalInput`
  (params (Direction :type "/Game/FencingGame/Fencer/E_Guards Enum" :default "NewEnumerator0"))
  ;[1 1 1] Input
  (if (not (`|EnumEquality` Direction (`/Game/FencingGame/Fencer/Animations/ABP_Fencer.GoalGuard` (`self.Anim`))))
    (`self.ServerGuardChange` Direction)))

(event `EnhancedInput|/Game/FencingGame/Fencer/Input/IA_Left`
  (params (ActionValue :type Boolean) (ElapsedSeconds :type "Float (double-precision)") (TriggeredSeconds :type "Float (double-precision)") (InputAction :type "InputAction Object Reference" :default "/Game/FencingGame/Fencer/Input/IA_Left.IA_Left"))
  ;[1 1 1] Input
  (:`Triggered`
    (`self.DirectionalInput` "NewEnumerator2")))

(event `EnhancedInput|/Game/FencingGame/Fencer/Input/IA_Up`
  (params (ActionValue :type Boolean) (ElapsedSeconds :type "Float (double-precision)") (TriggeredSeconds :type "Float (double-precision)") (InputAction :type "InputAction Object Reference" :default "/Game/FencingGame/Fencer/Input/IA_Up.IA_Up"))
  ;[1 1 1] Input
  (:`Triggered`
    (`self.DirectionalInput` "NewEnumerator1")))

(event `ServerGuardChange`
  (params (NewGuard :type "/Game/FencingGame/Fencer/E_Guards Enum" :default "NewEnumerator0"))
  ;[1 1 1] Input
  (if (`self.InputEnabled`)
    (`self.MulticastGuardChange` NewGuard)))

(event `MulticastBlocked`
  (bind _anim (`self.Anim`))
  (bind (_returnvalue_location _returnvalue_rotation _returnvalue_scale) (`KismetMathLibrary.BreakTransform` (`SceneComponent.K2_GetComponentToWorld` (`/Game/FencingGame/Fencer/BP_Fencer.BlockParticleLocation` (`self.Opponent`)))))
  ;[1 1 1] Block & Hit
  (set `/Game/FencingGame/Fencer/Animations/ABP_Fencer.Blocked` true _anim)
  (`NiagaraFunctionLibrary.SpawnSystemAtLocation` "/Game/sA_Megapack_v1/sA_StylizedAttacksPack/FX/NiagaraSystems/NS_BasicHit1.NS_BasicHit1" _returnvalue_location _returnvalue_rotation _returnvalue_scale)
  (`KismetSystemLibrary.Delay` 0.2)
  (set `/Game/FencingGame/Fencer/Animations/ABP_Fencer.Blocked` false _anim)
  (set `/Game/FencingGame/Fencer/Animations/ABP_Fencer.Swing` "NewEnumerator3" _anim))

(event `ServerSwing`
  (params (SwingDir :type "/Game/FencingGame/Fencer/E_Guards Enum" :default "NewEnumerator0"))
  ;[1 1 1] Input
  (if (`self.InputEnabled`)
    (if (`|EnumEquality` (`/Game/FencingGame/Fencer/Animations/ABP_Fencer.Swing` (`self.Anim`)) "NewEnumerator3")
      (`self.MulticastSwing` SwingDir))))

(event `MulticastGuardChange`
  (params (NewGuard :type "/Game/FencingGame/Fencer/E_Guards Enum" :default "NewEnumerator0"))
  (bind _anim (`self.Anim`))
  ;[1 1 1] Input
  (set `/Game/FencingGame/Fencer/Animations/ABP_Fencer.GoalGuard` NewGuard _anim)
  (if (and (`/Game/FencingGame/Fencer/Animations/ABP_Fencer.CanFeint` _anim) (`|EnumInequality` (`/Game/FencingGame/Fencer/Animations/ABP_Fencer.Swing` _anim) "NewEnumerator3"))
    (`/Game/FencingGame/Fencer/Animations/ABP_Fencer.AnimNotify_SwingEnd` _anim)))

(event `MulticastSwing`
  (params (SwingDir :type "/Game/FencingGame/Fencer/E_Guards Enum" :default "NewEnumerator0"))
  ;[1 1 1] Input
  (set `/Game/FencingGame/Fencer/Animations/ABP_Fencer.Swing` SwingDir (`self.Anim`)))

(event `MulticastHit`
  (bind _anim (`self.Anim`))
  ;[1 1 1] Block & Hit
  (set `/Game/FencingGame/Fencer/Animations/ABP_Fencer.Blocked` true _anim)
  (`KismetSystemLibrary.Delay` 0.2)
  (set `/Game/FencingGame/Fencer/Animations/ABP_Fencer.Blocked` false _anim)
  (set `/Game/FencingGame/Fencer/Animations/ABP_Fencer.Swing` "NewEnumerator3" _anim))

(event `EnhancedInput|/Game/FencingGame/Fencer/Input/IA_Attack`
  (params (ActionValue :type Boolean) (ElapsedSeconds :type "Float (double-precision)") (TriggeredSeconds :type "Float (double-precision)") (InputAction :type "InputAction Object Reference" :default "/Game/FencingGame/Fencer/Input/IA_Attack.IA_Attack"))
  (bind _endgamewidget (`self.EndGameWidget`))
  ;[1 1 1] Input
  (:`Triggered`
    (`/Engine/EditorBlueprintResources/StandardMacros.IsValid` _endgamewidget
      (:`Is Valid`
        (`/Game/FencingGame/UI/WBP_EndGame.ReadyForRematch` _endgamewidget))
      (:`Is Not Valid`
        (`self.ServerSwing` (`/Game/FencingGame/Fencer/Animations/ABP_Fencer.GoalGuard` (`self.Anim`)))))))

(event `Die`
  (bind _mesh (`self.Mesh`))
  ;[1 1 1] Block & Hit
  (set `self.IsDead` true)
  (set `self.InputEnabled` false)
  (`PrimitiveComponent.SetCollisionEnabled` _mesh "QueryAndPhysics")
  (`PrimitiveComponent.SetSimulatePhysics` _mesh true)
  (`PrimitiveComponent.AddImpulse` _mesh (* (`SceneComponent.GetForwardVector` (`self.RootComponent`)) -10000.0) "None" false))

(event `KillOpponent`
  ;[1 1 1] Block & Hit
  (set `self.InputEnabled` false))

(event `EnhancedInput|/Game/FencingGame/Fencer/Input/IA_MoveBackward`
  (params (ActionValue :type Boolean) (ElapsedSeconds :type "Float (double-precision)") (TriggeredSeconds :type "Float (double-precision)") (InputAction :type "InputAction Object Reference" :default "/Game/FencingGame/Fencer/Input/IA_MoveBackward.IA_MoveBackward"))
  ;[1 1 1] Movement
  (:`Triggered`
    (if (`self.InputEnabled`)
      (`self.AddMovementInput` (* (`self.GetActorForwardVector`) -1.0) 0.9))))

(event `EnhancedInput|/Game/FencingGame/Fencer/Input/IA_MoveForward`
  (params (ActionValue :type Boolean) (ElapsedSeconds :type "Float (double-precision)") (TriggeredSeconds :type "Float (double-precision)") (InputAction :type "InputAction Object Reference" :default "/Game/FencingGame/Fencer/Input/IA_MoveForward.IA_MoveForward"))
  ;[1 1 1] Movement
  (:`Triggered`
    (if (`self.InputEnabled`)
      (`self.AddMovementInput` (`self.GetActorForwardVector`)))))

(event `UpdateScore`
  (bind _asgm_fencing (cast `/Game/FencingGame/GameModes/GM_Fencing` (`GameplayStatics.GetGameMode`)))
  (`/Game/FencingGame/GameModes/GM_Fencing.ReportScore` _asgm_fencing (`self.GetController`))
  (`/Game/FencingGame/GameModes/GM_Fencing.PopulateScoreScreens` _asgm_fencing))

(event `RoundEndClient`
  (params (isVictory :type Boolean))
  (bind _returnvalue (`|CreateWidget` "/Game/FencingGame/UI/WBP_EndGame.WBP_EndGame_C" (`GameplayStatics.GetPlayerController` 0) isVictory))
  (bind _output_get (set `self.EndGameWidget` _returnvalue))
  (`UserWidget.AddToViewport` _output_get 0)
  (set `PlayerController.bShowMouseCursor` true (`GameplayStatics.GetPlayerController` 0)))

(event `ServerReadyForRematch`
  ; Match Flow
  (bind _asgm_fencing (cast `/Game/FencingGame/GameModes/GM_Fencing` (`GameplayStatics.GetGameMode`)))
  (bind _asplayer_controller (cast `PlayerController` (`self.GetController`)))
  (`/Game/FencingGame/GameModes/GM_Fencing.ReportReadyForRematch` _asgm_fencing _asplayer_controller))

(event `TakeStep`
  (params (isForward :type Boolean))
  ;[1 1 1] Movement
  (if (<= (`KismetMathLibrary.Vector_DistanceSquared` (`self.GoalPosition`) (`self.K2_GetActorLocation`)) 900.0)
    (set `self.GoalPosition` (+ (`self.GoalPosition`) (* (`self.GetActorForwardVector`) (`KismetMathLibrary.SelectFloat` 100.0 -100.0 isForward))))))

(event `ResetUI`
  ; Match Flow
  (set `self.EndGameWidget` null)
  (bind _foundwidgets (`WidgetBlueprintLibrary.GetAllWidgetsOfClass` "/Game/FencingGame/UI/WBP_EndGame.WBP_EndGame_C"))
  (for _array_element _foundwidgets
    (`Widget.RemoveFromParent` _array_element)))

(event `ServerEndSession`
  ; Match Flow
  (`self.MulticastEndSession`))

(event `MulticastEndSession`
  ; Match Flow
  (`DestroySessionCallbackProxy.DestroySession` (`GameplayStatics.GetPlayerController` 0)
    (:`OnSuccess`
      _)
    (:`OnFailure`
      _))
  (`GameplayStatics.OpenLevel` "MainMenu"))

(event `DisplayWaitingWidget`
  ; Match Flow
  (bind _returnvalue (`|CreateWidget` "/Game/FencingGame/UI/WBP_WaitingForOpp.WBP_WaitingForOpp_C" (`GameplayStatics.GetPlayerController` 0)))
  (bind _output_get (set `self.WaitingWidget` _returnvalue))
  (`UserWidget.AddToViewport` _output_get 0)
  (set `PlayerController.bShowMouseCursor` true (`GameplayStatics.GetPlayerController` 0)))

(event `MulticastStartGameUI`
  ; Match Flow
  (`/Engine/EditorBlueprintResources/StandardMacros.IsValid` (`self.WaitingWidget`)
    (:`Is Valid`
      (set `PlayerController.bShowMouseCursor` false (`GameplayStatics.GetPlayerController` 0))
      (`Widget.RemoveFromParent` (`self.WaitingWidget`))
      (set `self.WaitingWidget` null))
    (:`Is Not Valid`
      _))
  (bind _returnvalue (`|CreateWidget` "/Game/FencingGame/UI/WBP_StartGame.WBP_StartGame_C" (`GameplayStatics.GetPlayerController` 0)))
  (`UserWidget.AddToViewport` _returnvalue 0)
  (`KismetSystemLibrary.Delay` 0.7)
  (set `self.InputEnabled` true))

(event `EnhancedInput|/Game/FencingGame/Fencer/Input/IA_MainMenu`
  (params (ActionValue :type Boolean) (ElapsedSeconds :type "Float (double-precision)") (TriggeredSeconds :type "Float (double-precision)") (InputAction :type "InputAction Object Reference" :default "/Game/FencingGame/Fencer/Input/IA_MainMenu.IA_MainMenu"))
  (bind _endgamewidget (`self.EndGameWidget`))
  ; Match Flow
  (:`Triggered`
    (`/Engine/EditorBlueprintResources/StandardMacros.IsValid` _endgamewidget
      (:`Is Valid`
        (`/Game/FencingGame/UI/WBP_EndGame.GoToMainMenu` _endgamewidget)))))

(event `EnhancedInput|/Game/FencingGame/Fencer/Input/IA_RestartMatch`
  (params (ActionValue :type Boolean) (ElapsedSeconds :type "Float (double-precision)") (TriggeredSeconds :type "Float (double-precision)") (InputAction :type "InputAction Object Reference" :default "/Game/FencingGame/Fencer/Input/IA_RestartMatch.IA_RestartMatch"))
  ; Match Flow
)

(event `DisplayScore`
  (params (SelfScore :type Integer) (OpponentScore :type Integer))
  (bind _endgamewidget (`self.EndGameWidget`))
  (`/Engine/EditorBlueprintResources/StandardMacros.IsValid` _endgamewidget
    (:`Is Valid`
      (`/Game/FencingGame/UI/WBP_EndGame.DisplayScores` _endgamewidget SelfScore OpponentScore))
    (:`Is Not Valid`
      (`KismetSystemLibrary.PrintString` "Can't display scores, no end game widget"))))

(fn `UserConstructionScript`)