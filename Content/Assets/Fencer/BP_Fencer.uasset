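; BP_Fencer is a networked fencer character for directional melee duels with left, right and up guards.
; Directional input swings when it matches the current guard, otherwise changes guard, via Server-to-Multicast events that set ABP_Fencer variables.
; SwingConnect makes the server compare the swing to the opponent's mirrored guard, multicasting a block or hit.
; Blocks briefly flag the anim instance; the hit handler is empty and the swing reset is unconnected.
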(event `self.ReceiveBeginPlay`
  ;[1 1 1] Init
  (`|ExecutionSequence`
    (:`then_0`
      (`self.InitAnims`))
    (:`then_1`
      (`self.InitInput`))))

(event `InitAnims`
  ;[1 1 1] Init
  (bind _asabp_fencer (cast `/Game/Assets/Fencer/Animations/ABP_Fencer` (`SkeletalMeshComponent.GetAnimInstance` (`self.Mesh`))))
  (set `self.Anim` _asabp_fencer))

(event `InitInput`
  ;[1 1 1] Init
  (bind _asplayer_controller (cast `PlayerController` (`self.GetController`)))
  (`EnhancedInputSubsystemInterface.AddMappingContext` (pcsubsystem `EnhancedInputLocalPlayerSubsystem` _asplayer_controller) "/Game/Assets/Fencer/Input/IMC_Fencer.IMC_Fencer" 0 (struct)))

(event `EnhancedInput|/Game/Assets/Fencer/Input/IA_Right`
  (params (ActionValue :type Boolean) (ElapsedSeconds :type "Float (double-precision)") (TriggeredSeconds :type "Float (double-precision)") (InputAction :type "InputAction Object Reference" :default "/Game/Assets/Fencer/Input/IA_Right.IA_Right"))
  ;[1 1 1] Input
  (:`Triggered`
    (`self.DirectionalInput` "NewEnumerator0")))

(event `DirectionalInput`
  (params (Direction :type "/Game/Assets/Fencer/E_Guards Enum" :default "NewEnumerator0"))
  ;[1 1 1] Input
  (if (`|EnumEquality` Direction (`/Game/Assets/Fencer/Animations/ABP_Fencer.Guard` (`self.Anim`)))
    (`self.ServerSwing` Direction)
    (else
      (`self.ServerGuardChange` Direction))))

(event `EnhancedInput|/Game/Assets/Fencer/Input/IA_Left`
  (params (ActionValue :type Boolean) (ElapsedSeconds :type "Float (double-precision)") (TriggeredSeconds :type "Float (double-precision)") (InputAction :type "InputAction Object Reference" :default "/Game/Assets/Fencer/Input/IA_Left.IA_Left"))
  ;[1 1 1] Input
  (:`Triggered`
    (`self.DirectionalInput` "NewEnumerator2")))

(event `EnhancedInput|/Game/Assets/Fencer/Input/IA_Up`
  (params (ActionValue :type Boolean) (ElapsedSeconds :type "Float (double-precision)") (TriggeredSeconds :type "Float (double-precision)") (InputAction :type "InputAction Object Reference" :default "/Game/Assets/Fencer/Input/IA_Up.IA_Up"))
  ;[1 1 1] Input
  (:`Triggered`
    (`self.DirectionalInput` "NewEnumerator1")))

(event `ServerGuardChange`
  (params (NewGuard :type "/Game/Assets/Fencer/E_Guards Enum" :default "NewEnumerator0"))
  ;[1 1 1] Input
  (`self.MulticastGuardChange` NewGuard))

(event `ServerSwing`
  (params (SwingDir :type "/Game/Assets/Fencer/E_Guards Enum" :default "NewEnumerator0"))
  ;[1 1 1] Input
  (`self.MulticastSwing` SwingDir))

(event `MulticastGuardChange`
  (params (NewGuard :type "/Game/Assets/Fencer/E_Guards Enum" :default "NewEnumerator0"))
  ;[1 1 1] Input
  (set `/Game/Assets/Fencer/Animations/ABP_Fencer.Guard` NewGuard (`self.Anim`)))

(event `MulticastSwing`
  (params (SwingDir :type "/Game/Assets/Fencer/E_Guards Enum" :default "NewEnumerator0"))
  ;[1 1 1] Input
  (set `/Game/Assets/Fencer/Animations/ABP_Fencer.Swing` SwingDir (`self.Anim`)))

(event `SwingConnect`
  (`self.ServerTryHit`))

(event `ServerTryHit`
  (if (`|EnumEquality` (`/Game/Assets/Fencer/Animations/ABP_Fencer.Swing` (`self.Anim`)) (select `/Game/Assets/Fencer/E_Guards` (`/Game/Assets/Fencer/Animations/ABP_Fencer.Guard` (`/Game/Assets/Fencer/BP_Fencer.Anim` (`self.Opponent`))) :`NewEnumerator0` "NewEnumerator2" :`NewEnumerator1` "NewEnumerator1" :`NewEnumerator2` "NewEnumerator0" :`NewEnumerator3` "NewEnumerator3" :!type "/Game/Assets/Fencer/E_Guards Enum"))
    (`self.MulticastBlocked`)
    (else
      (`self.MulticastHit`))))

(event `MulticastHit`)

(event `MulticastBlocked`
  (bind _anim (`self.Anim`))
  (set `/Game/Assets/Fencer/Animations/ABP_Fencer.Blocked` true _anim)
  (`KismetSystemLibrary.Delay` 0.2)
  (set `/Game/Assets/Fencer/Animations/ABP_Fencer.Blocked` false _anim))

(fn `UserConstructionScript`)